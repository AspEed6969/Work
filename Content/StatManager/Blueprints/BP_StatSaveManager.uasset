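; BP_StatSaveManager is the persistence layer for stat managers, storing and restoring per-actor stats through a SaveGame_StatManager object.
; Assigning a stat first loads or creates that save object by slot name, then looks up the actor's entry.
; A found entry's stats and totals are copied onto the actor's stat manager and re-saved; otherwise the incoming stat is saved.
; Saving, lookup and removal delegate to the save object.
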(fn `Assign_StatManager`
  (params (Stat :type "/Game/StatManager/Blueprints/Data/Structures/Struct_StatSave Structure"))
  (`self.Check_For_Save_File`)
  (bind (_success _returnvalue) (`self.Load_Stat_Manager` (`.Actor_17_995819AA425B43F4681315BFC207D997` (break `/Game/StatManager/Blueprints/Data/Structures/Struct_StatSave` (`local.Stat`)))))
  (if _success
    (bind (_actor _stats _totalvalues) (break `/Game/StatManager/Blueprints/Data/Structures/Struct_StatSave` _returnvalue))
    (bind _returnvalue_2 (`/Game/StatManager/Blueprints/Data/FL_StatManager.Get_StatManager` _actor))
    (set `/Game/StatManager/Blueprints/Components/Manager_Stats.AvailableStats` _stats _returnvalue_2)
    (set `/Game/StatManager/Blueprints/Components/Manager_Stats.TotalValues` _totalvalues _returnvalue_2)
    (`self.Save_Stat_Manager` _returnvalue)
    (else
      (`self.Save_Stat_Manager` (`local.Stat`)))))

(fn `Check_For_Save_File`
  (bind _returnvalue (`GameplayStatics.DoesSaveGameExist` (`self.SaveFileName`)))
  (if _returnvalue
    (bind _returnvalue_2 (`GameplayStatics.LoadGameFromSlot` (`self.SaveFileName`)))
    (bind _assave_game_stat_manager (cast `/Game/StatManager/Blueprints/Data/SaveGames/SaveGame_StatManager` _returnvalue_2))
    (set `self.SaveGame` _assave_game_stat_manager)
    (else
      (bind _returnvalue_3 (`GameplayStatics.CreateSaveGameObject` "/Game/StatManager/Blueprints/Data/SaveGames/SaveGame_StatManager.SaveGame_StatManager_C"))
      (set `self.SaveGame` _returnvalue_3)))
  (set `/Game/StatManager/Blueprints/Data/SaveGames/SaveGame_StatManager.SaveSlotName` (`self.SaveFileName`) (`self.SaveGame`)))

(fn `Load_Stat_Manager`
  (params (Actor :type "Actor Object Reference"))
  (returns (Success :type Boolean) (ReturnValue :type "/Game/StatManager/Blueprints/Data/Structures/Struct_StatSave Structure"))
  (bind (_success _arrayindex _returnvalue) (`/Game/StatManager/Blueprints/Data/SaveGames/SaveGame_StatManager.Find_InSavedStats` (`self.SaveGame`) (`local.Actor`)))
  (return _success _returnvalue))

(fn `Remove_SavedStat`
  (params (Actor :type "Actor Object Reference"))
  (`/Game/StatManager/Blueprints/Data/SaveGames/SaveGame_StatManager.Remove_FromSavedStats` (`self.SaveGame`) (`local.Actor`)))

(fn `Save_Stat_Manager`
  (params (Stats :type "/Game/StatManager/Blueprints/Data/Structures/Struct_StatSave Structure"))
  (`/Game/StatManager/Blueprints/Data/SaveGames/SaveGame_StatManager.SaveStats` (`self.SaveGame`) (`local.Stats`)))

(fn `UserConstructionScript`)