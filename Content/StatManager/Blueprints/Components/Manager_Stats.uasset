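; Stat manager component that holds an actor's named stats, with functions to add, remove, reset, update and query them, firing dispatchers on changes.
; Static stats clamp to their limits, while Multiplied stats roll over like levels, rescaling max by a curve per step.
; A parallel TotalValues array tracks running totals and multiply counts.
; Changes are saved through the level's BP_StatSaveManager, which drops the owner's entry on EndPlay.
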(fn `Add_Stat`
  (params (StatInfo :type "/Game/StatManager/Blueprints/Data/Structures/Struct_StatMaster Structure"))
  ;[1 1 1] Comment
  (if (not (`self.Find_Stat_By_Name` (`.StatName_2_170313F3405E8D67A8AA0DBEC95E0979` (break `/Game/StatManager/Blueprints/Data/Structures/Struct_StatMaster` (`local.StatInfo`)))))
    (`KismetArrayLibrary.Array_Add` (`self.AvailableStats`) (`local.StatInfo`))
    ;[1 1 1] Call On Stat Added
    (`self.OnStatAdded` (`.StatName_2_170313F3405E8D67A8AA0DBEC95E0979` (break `/Game/StatManager/Blueprints/Data/Structures/Struct_StatMaster` (`local.StatInfo`))))
    ;[1 1 1] Save Stat For Owner
    (bind _statsavemanager (`self.StatSaveManager`)
      (:`then`
        (`/Game/StatManager/Blueprints/BP_StatSaveManager.Save_Stat_Manager` _statsavemanager (make `/Game/StatManager/Blueprints/Data/Structures/Struct_StatSave` (`self.OwnerActor`) (`self.AvailableStats`) (`self.TotalValues`))))
      (:`else`))))

(fn `Clamp_StatsByDefaults`
  (locals (LocStat :type "/Game/StatManager/Blueprints/Data/Structures/Struct_StatMaster Structure") (LocIndex :type Integer))
  (bind ((`Values_16_8CE822DC48001A794A0E20A7FE04A3AB` _values) (`DefaultValues_15_5B3F21314B62127F046EACA64A0DEA00` _defaultvalues)) (break `/Game/StatManager/Blueprints/Data/Structures/Struct_StatMaster` (`local.LocStat`)))
  (bind (_value _minvalue _maxvalue) (break `/Game/StatManager/Blueprints/Data/Structures/Struct_StatValues` _defaultvalues))
  ;[1 1 1] Clamp/Set All Values With The Default Values
  (for (_array_element _array_index) (`self.AvailableStats`)
    (set `local.LocStat` _array_element)
    (set `local.LocIndex` _array_index)
    (bind _structout (setmembers `/Game/StatManager/Blueprints/Data/Structures/Struct_StatValues` :`StructRef` _values :`Value` (`KismetMathLibrary.FClamp` _value _minvalue _maxvalue) :`Min Value` _minvalue :`Max Value` _maxvalue))
    (bind _structout_2 (setmembers `/Game/StatManager/Blueprints/Data/Structures/Struct_StatMaster` :`StructRef` (`local.LocStat`) :`Values` _structout))
    (set `local.LocStat` _structout_2)
    (`KismetArrayLibrary.Array_Set` (`self.AvailableStats`) (`local.LocIndex`) (`local.LocStat`))))

(fn `Find_InTotalValues`
  (params (StatName :type Name))
  (returns (ArrayIndex :type Integer) (ReturnValue :type "/Game/StatManager/Blueprints/Data/Structures/Struct_TotalValues Structure"))
  (locals (LocReturn :type "/Game/StatManager/Blueprints/Data/Structures/Struct_TotalValues Structure") (LocIndex :type Integer) (LocMultiply :type Integer))
  ;[1 1 1] Find In Total Values
  (for (_array_element _array_index) (`self.TotalValues`)
    (if (== (`.StatName_2_5DB9CB214212473AF3D0118557B16B2B` (break `/Game/StatManager/Blueprints/Data/Structures/Struct_TotalValues` _array_element)) (`local.StatName`))
      (set `local.LocReturn` _array_element)
      (set `local.LocIndex` _array_index)
      (break)))
  (return (`local.LocIndex`) (`local.LocReturn`)))

(fn `Find_Stat_By_Name`
  (params (StatName :type Name))
  (returns (Success :type Boolean) (ReturnValue :type "/Game/StatManager/Blueprints/Data/Structures/Struct_StatMaster Structure") (ArrayIndex :type Integer))
  (locals (LocReturn :type "/Game/StatManager/Blueprints/Data/Structures/Struct_StatMaster Structure") (LocSuccess :type Boolean :default false) (LocIndex :type Integer))
  (for (_array_element _array_index) (`self.AvailableStats`)
    (set `local.LocIndex` _array_index)
    (if (== (`.StatName_2_170313F3405E8D67A8AA0DBEC95E0979` (break `/Game/StatManager/Blueprints/Data/Structures/Struct_StatMaster` _array_element)) (`local.StatName`))
      (set `local.LocReturn` _array_element)
      (set `local.LocSuccess` true)
      (break)))
  (return (`local.LocSuccess`) (`local.LocReturn`) (`local.LocIndex`)))

(fn `Get_Ratio`
  (params (Stats :type "Array of Name") (DividerStat :type Name))
  (returns (ReturnValue :type "Float (double-precision)"))
  (locals (LocStats :type "Float (double-precision)" :default 0.0) (LocDivider :type "Float (double-precision)"))
  (`|ExecutionSequence`
    (:`then_0`
      ;[1 1 1] Collect All Requested Stat Values
      (for _array_element (`local.Stats`)
        (set `local.LocStats` (+ (`local.LocStats`) (`.Value_5_F47873DC4D59CFFC05366988B4B6913B` (break `/Game/StatManager/Blueprints/Data/Structures/Struct_TotalValues` (`.ReturnValue` (`self.Find_InTotalValues` _array_element))))))))
    (:`then_1`
      ;[1 1 1] Find Divider
      (set `local.LocDivider` (`.Value_5_F47873DC4D59CFFC05366988B4B6913B` (break `/Game/StatManager/Blueprints/Data/Structures/Struct_TotalValues` (`.ReturnValue` (`self.Find_InTotalValues` (`local.DividerStat`)))))))
    (:`then_2`
      ;[1 1 1] Return Ratio
      (return (/ (`local.LocStats`) (`local.LocDivider`))))))

(fn `Get_Stat`
  (params (StatName :type Name))
  (returns (ReturnValue :type "/Game/StatManager/Blueprints/Data/Structures/Struct_StatMaster Structure"))
  (locals (LocReturn :type "/Game/StatManager/Blueprints/Data/Structures/Struct_StatMaster Structure") (LocSuccess :type Boolean :default false) (LocIndex :type Integer))
  (for _array_element (`self.AvailableStats`)
    (if (== (`.StatName_2_170313F3405E8D67A8AA0DBEC95E0979` (break `/Game/StatManager/Blueprints/Data/Structures/Struct_StatMaster` _array_element)) (`local.StatName`))
      (set `local.LocReturn` _array_element)
      (break)))
  (return (`local.LocReturn`)))

(fn `Get_Stat_Value`
  (params (StatName :type Name))
  (returns (ReturnValue :type "Float (double-precision)"))
  (locals (LocReturn :type "Float (double-precision)") (LocSuccess :type Boolean :default false) (LocIndex :type Integer))
  (for _array_element (`self.AvailableStats`)
    (bind ((`StatName_2_170313F3405E8D67A8AA0DBEC95E0979` _statname) (`Values_16_8CE822DC48001A794A0E20A7FE04A3AB` _values)) (break `/Game/StatManager/Blueprints/Data/Structures/Struct_StatMaster` _array_element))
    (if (== _statname (`local.StatName`))
      (set `local.LocReturn` (`.Value_5_E0B8F7CB407DF0F1F7D138857C584E21` (break `/Game/StatManager/Blueprints/Data/Structures/Struct_StatValues` _values)))
      (break)))
  (return (`local.LocReturn`)))

(fn `Get_StatPercent`
  (params (StatName :type Name))
  (returns (ReturnValue :type "Float (double-precision)"))
  (bind (_success _returnvalue) (`self.Find_Stat_By_Name` StatName))
  (bind (_value _minvalue _maxvalue) (break `/Game/StatManager/Blueprints/Data/Structures/Struct_StatValues` (`.Values_16_8CE822DC48001A794A0E20A7FE04A3AB` (break `/Game/StatManager/Blueprints/Data/Structures/Struct_StatMaster` _returnvalue))))
  ;[1 1 1] Get Stat Percent By Current Max Value
  (if _success
    (return (`KismetMathLibrary.NormalizeToRange` _value _minvalue _maxvalue))))

(fn `IsStatValid?`
  (params (StatName :type Name))
  (returns (ReturnValue :type Boolean))
  (locals (LocSuccess :type Boolean))
  (for _array_element (`self.AvailableStats`)
    (if (== (`.StatName_2_170313F3405E8D67A8AA0DBEC95E0979` (break `/Game/StatManager/Blueprints/Data/Structures/Struct_StatMaster` _array_element)) (`local.StatName`))
      (set `local.LocSuccess` true)
      (break)))
  (return (`local.LocSuccess`)))

(fn `On_Owner_Destroyed`
  (params (Actor :type "Actor Object Reference") (EndPlayReason :type "EEndPlayReason Enum" :default "Destroyed"))
  ;[1 1 1] Remove Saved Stat If Actor Gets Destroyed
  (bind _statsavemanager (`self.StatSaveManager`)
    (:`then`
      (`/Game/StatManager/Blueprints/BP_StatSaveManager.Remove_SavedStat` _statsavemanager (`local.Actor`)))
    (:`else`)))

(fn `Override_Stat_Value`
  (params (StatName :type Name) (NewValue :type "Float (double-precision)"))
  (locals (LocStat :type "/Game/StatManager/Blueprints/Data/Structures/Struct_StatMaster Structure") (LocStatIndex :type Integer :default 0))
  (bind ((`MinValue_12_A229F0684100778FA519F085220135C0` _minvalue)) (break `/Game/StatManager/Blueprints/Data/Structures/Struct_StatValues` (`.Values_16_8CE822DC48001A794A0E20A7FE04A3AB` (break `/Game/StatManager/Blueprints/Data/Structures/Struct_StatMaster` (`local.LocStat`)))))
  (`|ExecutionSequence`
    (:`then_0`
      ;[1 1 1] Reset Stat To Default
      (set `local.LocStat` (`.ReturnValue` (`self.Find_Stat_By_Name` (`local.StatName`))))
      (`self.Reset_Stat_To_Default` (`local.StatName`)))
    (:`then_1`
      ;[1 1 1] Update Stat With The New Value
      (`self.Update_Stat_Value` (`local.StatName`) (`KismetMathLibrary.FMax` (`KismetMathLibrary.Abs` (- (`local.NewValue`) _minvalue)) _minvalue) true))
    (:`then_2`
      ;[1 1 1] Save Stat Manager
      (bind _statsavemanager (`self.StatSaveManager`)
        (:`then`
          (`/Game/StatManager/Blueprints/BP_StatSaveManager.Save_Stat_Manager` _statsavemanager (make `/Game/StatManager/Blueprints/Data/Structures/Struct_StatSave` (`self.OwnerActor`) (`self.AvailableStats`) (`self.TotalValues`))))
        (:`else`)))))

(fn `ReceiveBeginPlay`
  (`|ExecutionSequence`
    (:`then_0`
      ;[1 1 1] Clamp All Stats With The Default Values And Add For Each One A Total Value
      (`self.Clamp_StatsByDefaults`)
      (for _array_element (`self.AvailableStats`)
        (bind ((`StatName_2_170313F3405E8D67A8AA0DBEC95E0979` _statname) (`Values_16_8CE822DC48001A794A0E20A7FE04A3AB` _values)) (break `/Game/StatManager/Blueprints/Data/Structures/Struct_StatMaster` _array_element))
        (`KismetArrayLibrary.Array_Add` (`self.TotalValues`) (make `/Game/StatManager/Blueprints/Data/Structures/Struct_TotalValues` _statname (`.Value_5_E0B8F7CB407DF0F1F7D138857C584E21` (break `/Game/StatManager/Blueprints/Data/Structures/Struct_StatValues` _values))))))
    (:`then_1`
      ;[1 1 1] Set Owner Actor And Bind EndPlay
      (bind _output_get (set `self.OwnerActor` (`self.GetOwner`)))
      (add `Actor.OnEndPlay` _output_get (`|CreateDelegate` :!event `On_Owner_Destroyed`)))
    (:`then_2`
      ;[1 1 1] Get Stat Save Manager
      (bind _returnvalue (`GameplayStatics.GetActorOfClass` "/Game/StatManager/Blueprints/BP_StatSaveManager.BP_StatSaveManager_C"))
      (bind _output_get_2 (set `self.StatSaveManager` _returnvalue))
      (`/Engine/EditorBlueprintResources/StandardMacros.IsValid` _output_get_2
        (:`Is Valid`
          (`/Game/StatManager/Blueprints/BP_StatSaveManager.Assign_StatManager` _output_get_2 (make `/Game/StatManager/Blueprints/Data/Structures/Struct_StatSave` (`self.OwnerActor`) (`self.AvailableStats`) (`self.TotalValues`))))))))

(fn `Remove_Stat`
  (params (StatName :type Name))
  (bind (_success _returnvalue _arrayindex) (`self.Find_Stat_By_Name` StatName))
  ;[1 1 1] Remove Requested Stat
  (if _success
    (`KismetArrayLibrary.Array_Remove` (`self.AvailableStats`) _arrayindex)
    ;[1 1 1] Call On Stat Removed
    (`self.OnStatRemoved` (`local.StatName`))
    ;[1 1 1] Save Stat For Owner
    (bind _statsavemanager (`self.StatSaveManager`)
      (:`then`
        (`/Game/StatManager/Blueprints/BP_StatSaveManager.Save_Stat_Manager` _statsavemanager (make `/Game/StatManager/Blueprints/Data/Structures/Struct_StatSave` (`self.OwnerActor`) (`self.AvailableStats`) (`self.TotalValues`))))
      (:`else`))))

(fn `Reset_Stat_To_Default`
  (params (StatName :type Name))
  (locals (LocStat :type "/Game/StatManager/Blueprints/Data/Structures/Struct_StatMaster Structure"))
  (bind (_success _returnvalue _arrayindex) (`self.Find_Stat_By_Name` StatName))
  (bind (_arrayindex_2 _returnvalue_2) (`self.Find_InTotalValues` (`local.StatName`)))
  ;[1 1 1] Reset Stat Value To Defaults
  (if _success
    (set `local.LocStat` _returnvalue)
    (bind _structout (setmembers `/Game/StatManager/Blueprints/Data/Structures/Struct_StatMaster` :`StructRef` (`local.LocStat`) :`Values` (`.DefaultValues_15_5B3F21314B62127F046EACA64A0DEA00` (break `/Game/StatManager/Blueprints/Data/Structures/Struct_StatMaster` _returnvalue))))
    (`KismetArrayLibrary.Array_Set` (`self.AvailableStats`) _arrayindex _structout)
    ;[1 1 1] Reset Total Values
    (bind _structout_2 (setmembers `/Game/StatManager/Blueprints/Data/Structures/Struct_TotalValues` :`StructRef` _returnvalue_2 :`Value` (`.Value_5_E0B8F7CB407DF0F1F7D138857C584E21` (break `/Game/StatManager/Blueprints/Data/Structures/Struct_StatValues` (`.DefaultValues_15_5B3F21314B62127F046EACA64A0DEA00` (break `/Game/StatManager/Blueprints/Data/Structures/Struct_StatMaster` (`local.LocStat`))))) :`Multiply Count` 0))
    (`KismetArrayLibrary.Array_Set` (`self.TotalValues`) _arrayindex_2 _structout_2)
    ;[1 1 1] Call Dispatcher Event
    (`self.OnStatResetted` (`local.StatName`))
    ;[1 1 1] Save Stat For Owner
    (bind _statsavemanager (`self.StatSaveManager`)
      (:`then`
        (`/Game/StatManager/Blueprints/BP_StatSaveManager.Save_Stat_Manager` _statsavemanager (make `/Game/StatManager/Blueprints/Data/Structures/Struct_StatSave` (`self.OwnerActor`) (`self.AvailableStats`) (`self.TotalValues`))))
      (:`else`))))

(fn `Update_Stat_Value`
  (params (StatName :type Name) (Value :type "Float (double-precision)") (Increase :type Boolean))
  (locals (LocStatInfo :type "/Game/StatManager/Blueprints/Data/Structures/Struct_StatMaster Structure" :default (struct :`StatMultiplierType` "NewEnumerator0" :`Values` (struct :`MaxValue` 50.0) :`DefaultValues` (struct :`MaxValue` 50.0))) (LocStatIndex :type Integer :default 0) (LocStatName :type Name :default "None") (LocTotalValueIndex :type Integer :default 0) (LocTotalValues :type "/Game/StatManager/Blueprints/Data/Structures/Struct_TotalValues Structure") (LocCurrentValue :type "Float (double-precision)") (LocCurrentMinValue :type "Float (double-precision)") (LocCurrentMaxValue :type "Float (double-precision)") (LocNewValue :type "Float (double-precision)") (LocNewMaxValue :type "Float (double-precision)") (LocCurve :type "CurveFloat Object Reference") (LocCurrentMultiply :type Integer) (LocStartMultiplier :type Integer :default 0))
  (bind ((`Value_5_F47873DC4D59CFFC05366988B4B6913B` _value)) (break `/Game/StatManager/Blueprints/Data/Structures/Struct_TotalValues` (`local.LocTotalValues`)))
  (bind ((`Value_5_F47873DC4D59CFFC05366988B4B6913B` _value_2)) (break `/Game/StatManager/Blueprints/Data/Structures/Struct_TotalValues` (`local.LocTotalValues`)))
  (bind ((`StatName_2_170313F3405E8D67A8AA0DBEC95E0979` _statname) (`MultiplierCurve_18_DA7C466A49F1D5CA64CD7294BE5BB283` _multipliercurve)) (break `/Game/StatManager/Blueprints/Data/Structures/Struct_StatMaster` (`local.LocStatInfo`)))
  (bind (_values_value _values_minvalue _values_maxvalue) (break `/Game/StatManager/Blueprints/Data/Structures/Struct_StatValues` (break `/Game/StatManager/Blueprints/Data/Structures/Struct_StatMaster` (`local.LocStatInfo`))))
  (bind (_success _returnvalue _arrayindex) (`self.Find_Stat_By_Name` (`local.StatName`)))
  (bind (_arrayindex_2 _returnvalue_2) (`self.Find_InTotalValues` (`local.LocStatName`)))
  (bind (_value_3 _minvalue _maxvalue) (break `/Game/StatManager/Blueprints/Data/Structures/Struct_StatValues` (`.Values_16_8CE822DC48001A794A0E20A7FE04A3AB` (break `/Game/StatManager/Blueprints/Data/Structures/Struct_StatMaster` (`local.LocStatInfo`)))))
  (bind ((`MinValue_12_A229F0684100778FA519F085220135C0` _minvalue_2) (`MaxValue_6_FF09341641ED84B117A08F9173856D7A` _maxvalue_2)) (break `/Game/StatManager/Blueprints/Data/Structures/Struct_StatValues` (`.Values_16_8CE822DC48001A794A0E20A7FE04A3AB` (break `/Game/StatManager/Blueprints/Data/Structures/Struct_StatMaster` (`local.LocStatInfo`)))))
  (bind ((`MinValue_12_A229F0684100778FA519F085220135C0` _minvalue_3) (`MaxValue_6_FF09341641ED84B117A08F9173856D7A` _maxvalue_3)) (break `/Game/StatManager/Blueprints/Data/Structures/Struct_StatValues` (`.DefaultValues_15_5B3F21314B62127F046EACA64A0DEA00` (break `/Game/StatManager/Blueprints/Data/Structures/Struct_StatMaster` (`local.LocStatInfo`)))))
  (bind ((`MinValue_12_A229F0684100778FA519F085220135C0` _minvalue_4)) (break `/Game/StatManager/Blueprints/Data/Structures/Struct_StatValues` (`.DefaultValues_15_5B3F21314B62127F046EACA64A0DEA00` (break `/Game/StatManager/Blueprints/Data/Structures/Struct_StatMaster` (`local.LocStatInfo`)))))
  (bind (_value_4 _minvalue_5 _maxvalue_4) (break `/Game/StatManager/Blueprints/Data/Structures/Struct_StatValues` (`.Values_16_8CE822DC48001A794A0E20A7FE04A3AB` (break `/Game/StatManager/Blueprints/Data/Structures/Struct_StatMaster` (`local.LocStatInfo`)))))
  (bind _returnvalue_3 (`KismetMathLibrary.SelectFloat` (+ (`local.LocCurrentValue`) (`local.Value`)) (- (`local.LocCurrentValue`) (`local.Value`)) (`local.Increase`)))
  (`|ExecutionSequence`
    (:`then_0`
      ;[1 1 1] Cache Variables To Use In The Graph
      (if _success
        (set `local.LocStatInfo` _returnvalue)
        (set `local.LocStatIndex` _arrayindex)
        (set `local.LocStatName` _statname)
        (set `local.LocCurve` (select `bool` (`KismetSystemLibrary.IsValid` _multipliercurve) :`false` "/Game/StatManager/Blueprints/Data/Curves/Curve_StaticOneMultiplier.Curve_StaticOneMultiplier" :`true` _multipliercurve))
        (set `local.LocCurrentValue` _value_4)
        (set `local.LocCurrentMinValue` _minvalue_5)
        (set `local.LocCurrentMaxValue` _maxvalue_4)
        (set `local.LocTotalValueIndex` _arrayindex_2)
        (bind _output_get (set `local.LocTotalValues` _returnvalue_2))
        (bind _output_get_2 (set `local.LocCurrentMultiply` (`.MultiplyCount_10_58DB2C9548B608E1F71E099305F2A1C3` (break `/Game/StatManager/Blueprints/Data/Structures/Struct_TotalValues` _output_get))))
        (set `local.LocStartMultiplier` _output_get_2)))
    (:`then_1`
      ;[1 1 1] Switch On Stat Type
      (switch `/Game/StatManager/Blueprints/Data/Enums/Enum_StatType` (`.StatMultiplierType_11_36C0641E4614C71EC3A0D7B29B351083` (break `/Game/StatManager/Blueprints/Data/Structures/Struct_StatMaster` (`local.LocStatInfo`)))
        (:`NewEnumerator0`
          ;[1 1 1] Prevent Going Too Low Or High
          (if (`local.Increase`)
            (if (!= _maxvalue 0.0)
              (if (!= _value_3 _maxvalue)
                ;[1 1 1] Set New Value
                (set `local.LocNewValue` (`KismetMathLibrary.SelectFloat` (`KismetMathLibrary.FClamp` _returnvalue_3 _minvalue_2 _maxvalue_2) (`KismetMathLibrary.FMax` _returnvalue_3 _minvalue_2) (!= _maxvalue_2 0.0)) :!label _label)
                ;[1 1 1] Update Stat Value
                (bind _structout (setmembers `/Game/StatManager/Blueprints/Data/Structures/Struct_StatValues` :`StructRef` (`.Values_16_8CE822DC48001A794A0E20A7FE04A3AB` (break `/Game/StatManager/Blueprints/Data/Structures/Struct_StatMaster` (`local.LocStatInfo`))) :`Value` (`local.LocNewValue`)))
                (bind _structout_2 (setmembers `/Game/StatManager/Blueprints/Data/Structures/Struct_StatMaster` :`StructRef` (`local.LocStatInfo`) :`Values` _structout))
                (set `local.LocStatInfo` _structout_2)
                (`KismetArrayLibrary.Array_Set` (`self.AvailableStats`) (`local.LocStatIndex`) (`local.LocStatInfo`))
                ;[1 1 1] Update Total Value
                (bind _structout_3 (setmembers `/Game/StatManager/Blueprints/Data/Structures/Struct_TotalValues` :`StructRef` (`local.LocTotalValues`) :`Value` (`KismetMathLibrary.FMax` (`KismetMathLibrary.SelectFloat` (+ _value (`local.Value`)) (- _value (`local.Value`)) (`local.Increase`)))))
                (`KismetArrayLibrary.Array_Set` (`self.TotalValues`) (`local.LocTotalValueIndex`) _structout_3)
                ;[1 1 1] Call On Stat Updated
                (`self.OnStatUpdated` (`local.LocStatName`) (`local.LocNewValue`))
                ;[1 1 1] Trigger Event Dispatchers Based On The New Value
                (if (== _values_value _values_minvalue)
                  (`self.OnStatReachedToMin` (`local.LocStatName`))
                  (elif (and (== _values_value _values_maxvalue) (!= _values_maxvalue 0.0))
                    (`self.OnStatReachedToMax` (`local.LocStatName`)))))
              (else
                (goto _label)))
            (elif (!= _value_3 _minvalue)
              (goto _label))))
        (:`NewEnumerator1`
          ;[1 1 1] Increase?
          (if (`local.Increase`)
            ;[1 1 1] Update Total Value
            (bind _structout_4 (setmembers `/Game/StatManager/Blueprints/Data/Structures/Struct_TotalValues` :`StructRef` (`local.LocTotalValues`) :`Value` (`KismetMathLibrary.FMax` (+ (`.Value_5_F47873DC4D59CFFC05366988B4B6913B` (break `/Game/StatManager/Blueprints/Data/Structures/Struct_TotalValues` (`local.LocTotalValues`))) (`local.Value`)))))
            (`KismetArrayLibrary.Array_Set` (`self.TotalValues`) (`local.LocTotalValueIndex`) _structout_4)
            ;[1 1 1] Increase On Going Stat
            (`|ExecutionSequence`
              (:`then_0`
                (set `local.LocNewValue` (+ (`local.LocCurrentValue`) (`local.Value`)))
                (set `local.LocNewMaxValue` (`local.LocCurrentMaxValue`))
                (if (>= (`local.LocNewValue`) (`local.LocNewMaxValue`)) :!label _label_2
                  (set `local.LocNewValue` (`KismetMathLibrary.Conv_IntToDouble` (`KismetMathLibrary.Round` (- (`local.LocNewValue`) (`local.LocNewMaxValue`)))))
                  (set `local.LocNewMaxValue` (`KismetMathLibrary.Conv_IntToDouble` (`KismetMathLibrary.Round` (* (`local.LocNewMaxValue`) (`CurveFloat.GetFloatValue` (`local.LocCurve`) (`KismetMathLibrary.Conv_IntToDouble` (`local.LocCurrentMultiply`)))))))
                  (`/Engine/EditorBlueprintResources/StandardMacros.IncrementInt` (`local.LocCurrentMultiply`)
                    (:`  `
                      (goto _label_2)))))
              (:`then_1`
                ;[1 1 1] Update Stat Info
                (bind _structout_5 (setmembers `/Game/StatManager/Blueprints/Data/Structures/Struct_StatValues` :`StructRef` (`.Values_16_8CE822DC48001A794A0E20A7FE04A3AB` (break `/Game/StatManager/Blueprints/Data/Structures/Struct_StatMaster` (`local.LocStatInfo`))) :`Value` (`KismetMathLibrary.Conv_IntToDouble` (`KismetMathLibrary.Round` (`local.LocNewValue`))) :`Max Value` (`KismetMathLibrary.Conv_IntToDouble` (`KismetMathLibrary.Round` (`local.LocNewMaxValue`))) :!label _label_3))
                (bind _structout_6 (setmembers `/Game/StatManager/Blueprints/Data/Structures/Struct_StatMaster` :`StructRef` (`local.LocStatInfo`) :`Values` _structout_5))
                (set `local.LocStatInfo` _structout_6)
                (`KismetArrayLibrary.Array_Set` (`self.AvailableStats`) (`local.LocStatIndex`) (`local.LocStatInfo`))
                (bind _structout_7 (setmembers `/Game/StatManager/Blueprints/Data/Structures/Struct_TotalValues` :`StructRef` (`local.LocTotalValues`) :`Multiply Count` (`local.LocCurrentMultiply`)))
                (`KismetArrayLibrary.Array_Set` (`self.TotalValues`) (`local.LocTotalValueIndex`) _structout_7)
                ;[1 1 1] Call On Stat Updated
                (`self.OnStatUpdated` (`local.LocStatName`) (`local.LocNewValue`))
                ;[1 1 1] Call Event Dispatchers
                (for _ (range 1 (+ (`KismetMathLibrary.Abs_Int` (- (`local.LocStartMultiplier`) (`local.LocCurrentMultiply`))) 1))
                  (if (`local.Increase`)
                    (`self.OnStatReachedToMax` (`local.StatName`))
                    (else
                      (`self.OnStatReachedToMin` (`local.StatName`)))))))
            (else
              ;[1 1 1] Update Total Value
              (if (!= _value_2 _minvalue_4)
                (bind _structout_8 (setmembers `/Game/StatManager/Blueprints/Data/Structures/Struct_TotalValues` :`StructRef` (`local.LocTotalValues`) :`Value` (`KismetMathLibrary.FMax` (- _value_2 (`KismetMathLibrary.FClamp` (`local.Value`) 0.0 _value_2)) _minvalue_4)))
                (`KismetArrayLibrary.Array_Set` (`self.TotalValues`) (`local.LocTotalValueIndex`) _structout_8)
                ;[1 1 1] Decrease On Going Stat
                (`|ExecutionSequence`
                  (:`then_0`
                    (set `local.LocNewValue` (- (`local.LocCurrentValue`) (`local.Value`)))
                    (set `local.LocNewMaxValue` (`local.LocCurrentMaxValue`))
                    (if (< (`local.LocNewValue`) 0.0) :!label _label_4
                      (if (!= (`local.LocNewMaxValue`) (`.MaxValue_6_FF09341641ED84B117A08F9173856D7A` (break `/Game/StatManager/Blueprints/Data/Structures/Struct_StatValues` (`.DefaultValues_15_5B3F21314B62127F046EACA64A0DEA00` (break `/Game/StatManager/Blueprints/Data/Structures/Struct_StatMaster` (`local.LocStatInfo`))))))
                        (set `local.LocNewMaxValue` (`KismetMathLibrary.Conv_IntToDouble` (`KismetMathLibrary.Round` (/ (`local.LocNewMaxValue`) (`CurveFloat.GetFloatValue` (`local.LocCurve`) (`KismetMathLibrary.Conv_IntToDouble` (- (`local.LocCurrentMultiply`) 1)))))))
                        (set `local.LocNewValue` (`KismetMathLibrary.Conv_IntToDouble` (`KismetMathLibrary.Round` (`KismetMathLibrary.SelectFloat` (`KismetMathLibrary.FMax` (`local.LocNewValue`) _minvalue_3) (- (`local.LocNewMaxValue`) (`KismetMathLibrary.Abs` (`local.LocNewValue`))) (== _maxvalue_3 (`local.LocNewMaxValue`))))))
                        (`/Engine/EditorBlueprintResources/StandardMacros.DecrementInt` (`local.LocCurrentMultiply`)
                          (:`  `
                            (goto _label_4)))
                        (else
                          (set `local.LocNewValue` (`KismetMathLibrary.FMax` (`local.LocNewValue`) (`.MinValue_12_A229F0684100778FA519F085220135C0` (break `/Game/StatManager/Blueprints/Data/Structures/Struct_StatValues` (`.DefaultValues_15_5B3F21314B62127F046EACA64A0DEA00` (break `/Game/StatManager/Blueprints/Data/Structures/Struct_StatMaster` (`local.LocStatInfo`)))))))))))
                  (:`then_1`
                    (goto _label_3)))))))))
    (:`then_2`
      ;[1 1 1] Save Stat For Owner
      (bind _statsavemanager (`self.StatSaveManager`)
        (:`then`
          (`/Game/StatManager/Blueprints/BP_StatSaveManager.Save_Stat_Manager` _statsavemanager (make `/Game/StatManager/Blueprints/Data/Structures/Struct_StatSave` (`self.OwnerActor`) (`self.AvailableStats`) (`self.TotalValues`))))
        (:`else`)))))