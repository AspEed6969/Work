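; Enemy character V2: an AI melee opponent with a floating health widget, stealth takedown and slow-motion kill cam.
; Pawn sensing sets a blackboard flag, AttackPlayer sphere-traces to deal random damage, and overlap volumes toggle takedown eligibility and health display.
; Damage plays hit reactions; low health triggers ragdoll death, stops AI logic and updates player kill stats.
; A lethal hit on the player's locked target briefly switches to the kill camera.
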(event `self.ReceiveBeginPlay`
  ;[1 1 1 1 50] Event BeginPlay
  (`|ExecutionSequence`
    (:`then_0`
      (bind _asthird_person_character (cast `/Game/ThirdPersonBP/Blueprints/ThirdPersonCharacter` (`GameplayStatics.GetPlayerCharacter` 0)))
      (set `self.Char Ref` _asthird_person_character))
    (:`then_1`
      (`self.UpdateHealth_WB` 0.0))))

(event `self.ReceiveTick`
  (params (DeltaSeconds :type "Float (single-precision)"))
  ;[1 1 1 1 50] Event Tick
  (`SceneComponent.K2_SetWorldRotation` (`self.TextHealth_WB`) (`KismetMathLibrary.FindLookAtRotation` (`SceneComponent.K2_GetComponentLocation` (`self.TextHealth_WB`)) (`self.K2_GetActorLocation` (`GameplayStatics.GetPlayerCameraManager` 0))) false false))

(event `KillCamEvent`
  ;[0.3229 0.01514 0.01808 1 42] TakingDamage
  ;;[0.1458 0 0.003164] Kill Cam
  (`/Engine/EditorBlueprintResources/StandardMacros.DoOnce` false :!label _label
    (:`Completed`
      (`self.Kill Cam`
        (:`Output`
          (if (not (`self.Is Dead`))
            (goto _label :!via `Reset`)))))))

(event `/Game/Animation/Structure/I_Character.Attack Coming From Player`
  (params (`Incoming Damage` :type "Float (double-precision)"))
  ;[0.3229 0.01514 0.01808 1 42] TakingDamage
  (bind _trigger_kill_cam_ (`self.Slow motion Conditions` `Incoming Damage`))
  (if _trigger_kill_cam_
    (`self.KillCamEvent`)))

(event `self.ReceiveAnyDamage`
  (params (Damage :type "Float (single-precision)") (DamageType :type "DamageType Object Reference") (InstigatedBy :type "Controller Object Reference") (DamageCauser :type "Actor Object Reference"))
  (bind _char_ref (`self.Char Ref`))
  ;[0.3229 0.01514 0.01808 1 42] TakingDamage
  (if (`self.Is Dead`)
    (`KismetSystemLibrary.PrintString` "apush merela")
    (else
      (bind _returnvalue (`self.PlayAnimMontage` (`KismetArrayLibrary.Array_Random` (`self.AnimMontages`))))
      (`|ExecutionSequence`
        (:`then_0`
          (`GameplayStatics.PlaySound2D` "/Game/Animation/Structure/Sounds/GettingHit_Cue.GettingHit_Cue" 1.0 1.0 0.0 null null))
        (:`then_1`
          (if (not (`self.Is Dead`))
            (bind _output_get (set `self.HealthV3` (`KismetMathLibrary.FClamp` (- (`self.HealthV3`) Damage) 0.0 (`self.Max Health`))))
            (bind _get_v2_health (`self.UpdateHealth_WB` _output_get))
            (`SceneComponent.SetVisibility` (`self.WB_EnemyHealthV2`) true false)
            (`|ExecutionSequence`
              (:`then_0`
                (`KismetSystemLibrary.Delay` _returnvalue)
                (`self.Char Ref`
                  (:`then`)
                  (:`else`
                    (`SceneComponent.SetVisibility` (`self.WB_EnemyHealthV2`) false false))))
              (:`then_1`
                (if (<= _get_v2_health 15.0)
                  (`GameplayStatics.SetGlobalTimeDilation` 0.5)
                  (`self.Enemy Death` :!label _label_2)
                  (`GameplayStatics.SetGlobalTimeDilation` 1.0)
                  (`/Game/StatManager/Blueprints/Components/Manager_Stats.Update_Stat_Value` (`/Game/ThirdPersonBP/Blueprints/ThirdPersonCharacter.Manager_Stats` _char_ref) "TargetKilled" (+ (`self.KilledTargetsValue`) 1.0) true)
                  (`/Game/ThirdPersonBP/Blueprints/ThirdPersonCharacter.TargetsKilled` _char_ref)
                  (`KismetSystemLibrary.Delay` 4.0)
                  (`self.K2_DestroyActor`)
                  (elif (== _get_v2_health 0.0)
                    (goto _label_2)))))))))))

(event `TurningOn Regdoll`
  (`PrimitiveComponent.SetSimulatePhysics` (`self.Mesh`) true))

(event `self.TakeDownArea.OnComponentBeginOverlap`
  (params (OverlappedComponent :type "PrimitiveComponent Object Reference") (OtherActor :type "Actor Object Reference") (OtherComp :type "PrimitiveComponent Object Reference") (OtherBodyIndex :type Integer) (bFromSweep :type Boolean) (SweepResult :type "HitResult Structure (by ref)"))
  ;[0.9566 1 0.08689 1 34] TakeDown
  (bind _asthird_person_character (cast `/Game/ThirdPersonBP/Blueprints/ThirdPersonCharacter` OtherActor))
  (set `/Game/ThirdPersonBP/Blueprints/ThirdPersonCharacter.CanTakeDown?` true _asthird_person_character))

(event `self.PawnSensing.OnSeePawn`
  (params (Pawn :type "Pawn Object Reference"))
  ;[0.4385 1 0.6211] Attacking Player
  ;;[1 1 1] Saw The Player
  (cast `/Game/ThirdPersonBP/Blueprints/ThirdPersonCharacter` Pawn)
  (`BlackboardComponent.SetValueAsBool` (`AIBlueprintHelperLibrary.GetBlackboard` (`AIBlueprintHelperLibrary.GetAIController` self)) "HasSeenPlayer?" true))

(event `self.TakeDownArea.OnComponentEndOverlap`
  (params (OverlappedComponent :type "PrimitiveComponent Object Reference") (OtherActor :type "Actor Object Reference") (OtherComp :type "PrimitiveComponent Object Reference") (OtherBodyIndex :type Integer))
  ;[0.9566 1 0.08689 1 34] TakeDown
  (bind _asthird_person_character (cast `/Game/ThirdPersonBP/Blueprints/ThirdPersonCharacter` OtherActor))
  (set `/Game/ThirdPersonBP/Blueprints/ThirdPersonCharacter.CanTakeDown?` false _asthird_person_character))

(event `Attack Player`
  (bind _returnvalue (`self.K2_GetActorLocation`))
  ;[0.4385 1 0.6211] Attacking Player
  (if (`self.Is Dead`)
    (`KismetSystemLibrary.PrintString` "merel es debilot")
    (else
      (bind (_outhit _returnvalue_2) (`KismetSystemLibrary.SphereTraceSingleForObjects` _returnvalue (+ _returnvalue (* (`KismetMathLibrary.GetForwardVector` (`self.K2_GetActorRotation`)) 35.0)) 50.0 (`|MakeArray` "ObjectTypeQuery3" :!type "EObjectTypeQuery Enum")))
      (if _returnvalue_2
        (bind (_bblockinghit _binitialoverlap _time _distance _location _impactpoint _normal _impactnormal _physmat _hitactor) (`GameplayStatics.BreakHitResult` _outhit))
        (cast `/Game/ThirdPersonBP/Blueprints/ThirdPersonCharacter` _hitactor)
        (`self.PlayAnimMontage` self "/Game/Animation/BP/NewMesh/Anims/AnimMontages/Hookpunch_UE_Montage.Hookpunch_UE_Montage" 1.0 "None")
        (`GameplayStatics.ApplyDamage` _hitactor (`KismetMathLibrary.Conv_IntToDouble` (`KismetMathLibrary.Round` (`KismetMathLibrary.RandomFloatInRange` 10.0 20.0))))
        (`GameplayStatics.SpawnEmitterAtLocation` "/Game/Realistic_Starter_VFX_Pack_Vol2/Particles/Blood/P_Blood_Splat_Cone.P_Blood_Splat_Cone" (+ _location (0.0 100.0 15.0)) (`KismetArrayLibrary.Array_Random` (`|MakeArray` (`KismetMathLibrary.MakeRotFromXY` _normal _normal) (`KismetMathLibrary.MakeRotFromYZ` _normal _normal) (`KismetMathLibrary.MakeRotFromYX` _normal _normal) (`KismetMathLibrary.MakeRotFromZX` _normal _normal) (`KismetMathLibrary.MakeRotationFromAxes` _normal (10.0 15.0 5.0) (5.0 5.0 -5.0)))) (0.6 0.6 0.4))))))

(event `TakeDown`
  ;[0.9566 1 0.08689 1 34] TakeDown
  (`CharacterMovementComponent.DisableMovement` (`self.CharacterMovement`))
  (`self.DisableInput` null)
  (`self.SetActorEnableCollision` false)
  (`|PlayMontage` (`self.Mesh`) "/Game/Animation/BP/NewMesh/Anims/AnimMontages/StealthAssassination_Victim_UE_Montage.StealthAssassination_Victim_UE_Montage"
    (:`OnCompleted`
      (`self.K2_DestroyActor`))))

(event `self.Sphere.OnComponentBeginOverlap`
  (params (OverlappedComponent :type "PrimitiveComponent Object Reference") (OtherActor :type "Actor Object Reference") (OtherComp :type "PrimitiveComponent Object Reference") (OtherBodyIndex :type Integer) (bFromSweep :type Boolean) (SweepResult :type "HitResult Structure (by ref)"))
  (if (not (`self.Is Dead`))
    (bind _asthird_person_character (cast `/Game/ThirdPersonBP/Blueprints/ThirdPersonCharacter` OtherActor))
    (`/Engine/EditorBlueprintResources/StandardMacros.IsValid` _asthird_person_character
      (:`Is Valid`
        (`SceneComponent.SetVisibility` (`self.WB_EnemyHealthV2`) true false)))))

(event `self.Sphere.OnComponentEndOverlap`
  (params (OverlappedComponent :type "PrimitiveComponent Object Reference") (OtherActor :type "Actor Object Reference") (OtherComp :type "PrimitiveComponent Object Reference") (OtherBodyIndex :type Integer))
  (if (not (`self.Is Dead`))
    (bind _asthird_person_character (cast `/Game/ThirdPersonBP/Blueprints/ThirdPersonCharacter` OtherActor))
    (`/Engine/EditorBlueprintResources/StandardMacros.IsValid` _asthird_person_character
      (:`Is Valid`
        (`SceneComponent.SetVisibility` (`self.WB_EnemyHealthV2`) false false)))))

(fn `Enemy Death`
  (bind _returnvalue (`AIBlueprintHelperLibrary.GetAIController` (`self.GetController`)))
  (set `self.Is Dead` true)
  (`self.Mesh`
    (:`then`
      (`|ExecutionSequence`
        (:`then_0`
          (`PrimitiveComponent.SetSimulatePhysics` (`self.Mesh`) true)
          (`PrimitiveComponent.SetCollisionEnabled` (`self.CapsuleComponent`) "NoCollision")
          (`ActorComponent.K2_DestroyComponent` (`self.CapsuleComponent`))
          (`/Engine/EditorBlueprintResources/StandardMacros.IsValid` _returnvalue
            (:`Is Valid`
              (`BrainComponent.StopLogic` (`AIController.BrainComponent` _returnvalue) ""))
            (:`Is Not Valid`
              _))
          (`PrimitiveComponent.SetCollisionObjectType` (`self.Mesh`) "ECC_Pawn")
          (`/Game/Animation/Structure/I_Character.Remove Lock ON` (`self.Char Ref`))
          (`ActorComponent.K2_DestroyComponent` (`self.WB_EnemyHealthV2`))
          (`SkeletalMeshComponent.SetAnimationMode` (`self.Mesh`) "AnimationCustomMode")
          (return))
        (:`then_1`
          (`ActorComponent.K2_DestroyComponent` (`self.CapsuleComponent`)))))
    (:`else`)))

(fn `GetWeaponSocket`
  (params (`Socket Name` :type Name))
  (returns (LeftHandLocation :type "Transform Structure"))
  (return))

(fn `Slow motion Conditions`
  (params (`Incoming Damage` :type "Float (double-precision)"))
  (returns (`Trigger Kill Cam?` :type Boolean))
  (if (== (`/Game/ThirdPersonBP/Blueprints/ThirdPersonCharacter.Locked Target` (`self.Char Ref`)) self)
    (if (`self.Is Dead`)
      (set `self.CanTriggerKIllCam` false :!label _label)
      (elif (>= `Incoming Damage` (`self.HealthV3`))
        (bind _output_get (set `self.CanTriggerKIllCam` true))
        (else
          (goto _label))))
    (else
      (goto _label)))
  (return _output_get))

(fn `Slow motion Running`
  (params (Condition :type Boolean))
  (if Condition
    (set `self.SlowMotionOccuring` true)
    (`self.DisableInput` (`self.Char Ref`) (`GameplayStatics.GetPlayerController` 0))
    (else
      (`self.EnableInput` (`self.Char Ref`) (`GameplayStatics.GetPlayerController` 0))
      (set `self.SlowMotionOccuring` false))))

(fn `UpdateHealth_WB`
  (params (V2_Health :type "Float (single-precision)"))
  (returns (Get_V2_Health :type "Float (single-precision)"))
  (bind _asenemy_health_v2_wb (cast `/Game/Enemy/EnemyV2/EnemyHealthV2_WB` (`WidgetComponent.GetUserWidgetObject` (`self.WB_EnemyHealthV2`))))
  (bind _output_get (set `/Game/Enemy/EnemyV2/EnemyHealthV2_WB.V2_Health` (`self.HealthV3`) _asenemy_health_v2_wb))
  (return _output_get))

(fn `UserConstructionScript`)