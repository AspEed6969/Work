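; Player HUD that draws a lock-on reticle over the enemy the player's ThirdPersonCharacter has targeted.
; BeginPlay caches the character reference, and Tick toggles the reticle size between visible and zero based on its TargetLock flag and a valid LockedTarget.
; DrawHUD projects the target's world location to screen space and draws the target texture there with a small pixel offset.
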(event `self.ReceiveBeginPlay`
  (bind _asthird_person_character (cast `/Game/ThirdPersonBP/Blueprints/ThirdPersonCharacter` (`GameplayStatics.GetPlayerCharacter` 0)))
  (set `self.Char Ref` _asthird_person_character))

(event `self.ReceiveDrawHUD`
  (params (SizeX :type Integer) (SizeY :type Integer))
  (bind _targetscale (`self.TargetScale`))
  (bind _locked_target (`/Game/ThirdPersonBP/Blueprints/ThirdPersonCharacter.Locked Target` (`self.Char Ref`)))
  (bind _screenlocation (`PlayerController.ProjectWorldLocationToScreen` (`GameplayStatics.GetPlayerController` 0) (`self.K2_GetActorLocation` _locked_target) false))
  (`/Engine/EditorBlueprintResources/StandardMacros.IsValid` _locked_target
    (:`Is Valid`
      (`self.DrawTexture` "/Game/Enemy/EnemyV2/T_target.T_target" (- (`KismetMathLibrary.BreakVector2D` _screenlocation) 7.0) (- (`.Y` (`KismetMathLibrary.BreakVector2D` _screenlocation)) 23.0) _targetscale _targetscale 0.0 0.0 1.0 1.0))))

(event `self.ReceiveTick`
  (params (DeltaSeconds :type "Float (single-precision)"))
  (bind _char_ref (`self.Char Ref`))
  (`/Engine/EditorBlueprintResources/StandardMacros.IsValid` (`self.Char Ref`)
    (:`Is Valid`
      (if (and (`/Game/ThirdPersonBP/Blueprints/ThirdPersonCharacter.TargetLock?` _char_ref) (`KismetSystemLibrary.IsValid` (`/Game/ThirdPersonBP/Blueprints/ThirdPersonCharacter.Locked Target` _char_ref)))
        (set `self.TargetScale` 13.0)
        (else
          (set `self.TargetScale` 0.0))))))

(fn `UserConstructionScript`)