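; Enemy Blueprint with a health widget component and a brief collision-off window after taking damage.
; AnyDamage disables capsule collision, sets Health0 to damage minus one, caches the WB_EnemyHealth widget, then restores collision after 0.2 seconds.
; OnHeadPositionCalculated runs the same sequence after calling CreateDamageNumberWidget.
; OnTakeDamage and CreateDamageNumberWidget are stubs, with the latter's widget-spawning code unreachable.
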(event `OnHeadPositionCalculated`
  (params (`Head Position` :type "Vector Structure"))
  (`self.OnHeadPositionCalculated` `Head Position`)
  (`self.Create Damage Number Widget` (0.0 0.0 0.0))
  (`PrimitiveComponent.SetCollisionEnabled` (`self.CapsuleComponent`) "NoCollision" :!label _label)
  (set `self.Health_0` (- (stale `self.ReceiveAnyDamage` Damage) 1.0))
  (bind _aswb_enemy_health (cast `/Game/Enemy/WDB/WB_EnemyHealth` (`WidgetComponent.GetUserWidgetObject` (`self.Widget`))))
  (set `self.As WB Enemy Health` _aswb_enemy_health)
  (`KismetSystemLibrary.Delay` 0.2)
  (`PrimitiveComponent.SetCollisionEnabled` (`self.CapsuleComponent`) "QueryAndPhysics"))

(event `self.ReceiveAnyDamage`
  (params (Damage :type "Float (single-precision)") (DamageType :type "DamageType Object Reference") (InstigatedBy :type "Controller Object Reference") (DamageCauser :type "Actor Object Reference"))
  (goto _label))

(fn `Create Damage Number Widget`
  (params (NewParam :type "Vector Structure"))
  (returns (NewParam1 :type "Widget Object Reference"))
  (return null))

(fn `OnTakeDamage`
  (params (NewParam :type "Float (double-precision)"))
  (returns (Actor :type "Actor Object Reference"))
  (return null))

(fn `UserConstructionScript`)