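; Rifle actor that the third-person character can pick up, holding its own ammo and reload logic.
; Sphere overlap registers it as the character's NearWeaponRifle, and PickUpRifle destroys it a tick later.
; Reload plays a rifle montage, then clears the character's Reloading flag and refills Bullets from Magazine, which acts as the reserve.
; Interact events and InteractRep's OnRep are empty; widget and mesh setup are unconnected.
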(event `/Game/Animation/Structure/I_Items.Pick Up Rifle`
  (`KismetSystemLibrary.DelayUntilNextTick`)
  (`self.K2_DestroyActor`)
  (bind _asthird_person_character (cast `/Game/ThirdPersonBP/Blueprints/ThirdPersonCharacter` (stale `self.Sphere.OnComponentBeginOverlap` OtherActor) :!label _label))
  (bind _output_get (set `self.Char Ref` _asthird_person_character))
  (set `/Game/ThirdPersonBP/Blueprints/ThirdPersonCharacter.Near Weapon_Rifle` self _output_get))

(event `self.Sphere.OnComponentBeginOverlap`
  (params (OverlappedComponent :type "PrimitiveComponent Object Reference") (OtherActor :type "Actor Object Reference") (OtherComp :type "PrimitiveComponent Object Reference") (OtherBodyIndex :type Integer) (bFromSweep :type Boolean) (SweepResult :type "HitResult Structure (by ref)"))
  (`|ExecutionSequence`
    (:`then_0`
      (goto _label))))

(event `Reload`
  (bind _magazine (`self.Magazine`))
  (bind _maxbullets (`self.MaxBullets`))
  (if (> (`self.Magazine`) 0.0)
    (`|PlayMontage` (`self.Rifle`) "/Game/Projectile/Rifle/Weapons/Anims/SK_Rifle_Reloading_Anim_Montage.SK_Rifle_Reloading_Anim_Montage" 1.0 0.0 "DefaultSlot"
      (:`OnCompleted`
        (set `/Game/ThirdPersonBP/Blueprints/ThirdPersonCharacter.Reloading` false (`self.Char Ref`))
        (if (> (`self.Magazine`) (`self.MaxBullets`))
          (set `self.Bullets` _maxbullets)
          (set `self.Magazine` (- (`self.Magazine`) _maxbullets))
          (else
            (set `self.Bullets` _magazine)
            (set `self.Magazine` (- _magazine _magazine))))))))

(event `/Game/Animation/Structure/I_Items.Interface Toggle Focus`
  (params (Focus :type Boolean)))

(event `/Game/Animation/Structure/I_Items.Interface Interact`)

(event `InteractOnServer`)

(fn `OnRep_InteractRep`)

(fn `UserConstructionScript`)