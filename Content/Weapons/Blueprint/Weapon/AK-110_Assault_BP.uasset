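; Weapon actor Blueprint for the AK-110 assault rifle that tracks the character touching it and can remove itself from the world.
; Its Sphere overlap casts the other actor to ThirdPersonCharacter and stores it as CharRef.
; A custom event waits one tick, destroys the actor, then runs into the same cast.
; Interact widget creation and the NearWeaponRifle assignment are left unconnected, and Tick is disabled.
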(event `CustomEvent`
  (`KismetSystemLibrary.DelayUntilNextTick`)
  (`self.K2_DestroyActor`)
  (bind _asthird_person_character (cast `/Game/ThirdPersonBP/Blueprints/ThirdPersonCharacter` (stale `self.Sphere.OnComponentBeginOverlap` OtherActor) :!label _label))
  (set `self.Char Ref` _asthird_person_character))

(event `self.Sphere.OnComponentBeginOverlap`
  (params (OverlappedComponent :type "PrimitiveComponent Object Reference") (OtherActor :type "Actor Object Reference") (OtherComp :type "PrimitiveComponent Object Reference") (OtherBodyIndex :type Integer) (bFromSweep :type Boolean) (SweepResult :type "HitResult Structure (by ref)"))
  (`|ExecutionSequence`
    (:`then_0`
      (goto _label))))

(fn `UserConstructionScript`
  (`parent.UserConstructionScript`))